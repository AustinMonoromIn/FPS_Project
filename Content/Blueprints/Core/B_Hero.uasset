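; B_Hero is the player hero Blueprint, handling movement, aiming and a debug health test.
; Input events drive jump, crouch and controller pitch/yaw, with rate-based look variants scaled by base rate and frame delta time for gamepads.
; MoveForward and MoveRight feed a constant scale into movement input rather than their axis values.
; The H key subtracts Health, prints it and sets IsDead once it reaches zero or below.
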(event `InputAction|Jump`
  (params (Key :type "Key Structure"))
  ;[1 1 1] Movement and Aiming
  (:`Pressed`
    (`self.Jump`)))

(event `Key|H`
  (params (Key :type "Key Structure"))
  ;[1 1 1] Health Testing/Logic
  (:`Pressed`
    (bind _output_get (set `self.Health` (- (`self.Health`) 17.0)))
    (`KismetSystemLibrary.PrintString` (`KismetStringLibrary.Conv_DoubleToString` _output_get))
    (if (<= _output_get 0.0)
      (bind _output_get_2 (set `self.IsDead?` true))
      (`KismetSystemLibrary.PrintString` (`KismetStringLibrary.Conv_BoolToString` _output_get_2)))))

(event `InputAction|Crouch`
  (params (Key :type "Key Structure"))
  ;[1 1 1] Movement and Aiming
  (:`Pressed`
    (`self.Crouch`))
  (:`Released`
    (`self.UnCrouch`)))

(event `InputAction|Action/Reload`
  (params (Key :type "Key Structure")))

(event `InputAction|SwitchWeapons`
  (params (Key :type "Key Structure")))

(event `InputAxis|MoveForward`
  (params (AxisValue :type "Float (single-precision)"))
  ;[1 1 1] Movement and Aiming
  (`self.AddMovementInput` (`self.GetActorForwardVector`)))

(event `InputAction|Fire`
  (params (Key :type "Key Structure")))

(event `InputAction|Aim`
  (params (Key :type "Key Structure")))

(event `InputAxis|MoveRight`
  (params (AxisValue :type "Float (single-precision)"))
  ;[1 1 1] Movement and Aiming
  (`self.AddMovementInput` (`self.GetActorRightVector`)))

(event `InputAxis|LookUp`
  (params (AxisValue :type "Float (single-precision)"))
  ;[1 1 1] Movement and Aiming
  (`self.AddControllerPitchInput` AxisValue))

(event `InputAxis|LookUpRate`
  (params (AxisValue :type "Float (single-precision)"))
  ;[1 1 1] Aiming (Gamepad)
  (`self.AddControllerPitchInput` (* AxisValue (`self.BaseLookUpRate`) (`GameplayStatics.GetWorldDeltaSeconds`))))

(event `InputAxis|LookRight`
  (params (AxisValue :type "Float (single-precision)"))
  ;[1 1 1] Movement and Aiming
  (`self.AddControllerYawInput` AxisValue))

(event `InputAxis|LookRightRate`
  (params (AxisValue :type "Float (single-precision)"))
  ;[1 1 1] Aiming (Gamepad)
  (`self.AddControllerYawInput` (* AxisValue (`self.BaseLookRightRate`) (`GameplayStatics.GetWorldDeltaSeconds`))))

(fn `UserConstructionScript`
  (`parent.UserConstructionScript`))