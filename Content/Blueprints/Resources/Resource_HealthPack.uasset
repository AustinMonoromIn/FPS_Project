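; Health pack pickup that restores a fixed amount of health to the hero on a key press while they stand in its trigger.
; Box overlap begin and end enable and disable player input on the actor for the hero only.
; The Reload action then heals only if health is missing, clamps to the hero's maximum, destroys the pack and prints the new health.
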(event `self.BoxTrigger.OnComponentBeginOverlap`
  (params (OverlappedComponent :type "PrimitiveComponent Object Reference") (OtherActor :type "Actor Object Reference") (OtherComp :type "PrimitiveComponent Object Reference") (OtherBodyIndex :type Integer) (bFromSweep :type Boolean) (SweepResult :type "HitResult Structure (by ref)"))
  ;[1 1 1] When hero collides with trigger, enable input
  (if (== OtherActor (`self.HeroReference`))
    (`self.EnableInput` (`GameplayStatics.GetPlayerController` 0))))

(event `InputAction|Action/Reload`
  (params (Key :type "Key Structure"))
  (bind _heroreference (`self.HeroReference`))
  (bind _heroreference_2 (`self.HeroReference`))
  ;[1 1 1] Health pack logic
  (:`Pressed`
    (if (< (`/Game/Blueprints/Core/B_BaseCharacter.HealthActual` _heroreference) (`/Game/Blueprints/Core/B_BaseCharacter.HealthMax` _heroreference))
      (bind _output_get (set `/Game/Blueprints/Core/B_BaseCharacter.HealthActual` (`KismetMathLibrary.FClamp` (+ (`/Game/Blueprints/Core/B_BaseCharacter.HealthActual` _heroreference_2) 25.0) 0.0 (`/Game/Blueprints/Core/B_BaseCharacter.HealthMax` _heroreference_2)) (`self.HeroReference`)))
      (`self.K2_DestroyActor`)
      (`KismetSystemLibrary.PrintString` (`KismetStringLibrary.Conv_DoubleToString` _output_get)))))

(event `self.BoxTrigger.OnComponentEndOverlap`
  (params (OverlappedComponent :type "PrimitiveComponent Object Reference") (OtherActor :type "Actor Object Reference") (OtherComp :type "PrimitiveComponent Object Reference") (OtherBodyIndex :type Integer))
  ;[1 1 1] When hero leaves collision, disable input
  (if (== OtherActor (`self.HeroReference`))
    (`self.DisableInput` (`GameplayStatics.GetPlayerController` 0))))

(fn `UserConstructionScript`
  (`parent.UserConstructionScript`))